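; BP_BaseInteractable is a base interactable actor that signals to the player when it is in range.
; Its InteractionSphere overlap events show a Billboard when a BP_BasePawn enters and hide it when one leaves.
; On BeginPlay it caches the BP_ICBW_PlayerController, and its Interact event plays a 2D sound.
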(event `self.ReceiveBeginPlay`
  (bind _asbp_icbw_player_controller (cast `/Game/Blueprints/Core/BP_ICBW_PlayerController` (`GameplayStatics.GetPlayerController` 0)))
  (set `self.PlayerControllerRef` _asbp_icbw_player_controller))

(event `self.ReceiveTick`
  (params (DeltaSeconds :type "Float (single-precision)")))

(event `self.InteractionSphere.OnComponentBeginOverlap`
  (params (OverlappedComponent :type "PrimitiveComponent Object Reference") (OtherActor :type "Actor Object Reference") (OtherComp :type "PrimitiveComponent Object Reference") (OtherBodyIndex :type Integer) (bFromSweep :type Boolean) (SweepResult :type "HitResult Structure (by ref)"))
  (cast `/Game/Blueprints/Pawns/BP_BasePawn` OtherActor)
  (`SceneComponent.SetVisibility` (`self.Billboard`) true false))

(event `self.InteractionSphere.OnComponentEndOverlap`
  (params (OverlappedComponent :type "PrimitiveComponent Object Reference") (OtherActor :type "Actor Object Reference") (OtherComp :type "PrimitiveComponent Object Reference") (OtherBodyIndex :type Integer))
  (cast `/Game/Blueprints/Pawns/BP_BasePawn` OtherActor)
  (`SceneComponent.SetVisibility` (`self.Billboard`) false false))

(event `/Game/Blueprints/Interfaces/BPI_Interaction.Interact`
  (`GameplayStatics.PlaySound2D` (`self.Sound`) 1.0 1.0 0.0 null null))

(fn `UserConstructionScript`)
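; Game mode that alternates play between Calm and Storm phases and raises Difficulty after each storm.
; A looping one-second timer runs UpdateTime, which counts down the current phase and flips PlayState at zero.
; Each flip notifies all actors implementing BPI_PlayStateEvents.
; After a storm, Difficulty-scaled adjustments apply to the spent counters without resetting them, so the next Calm starts at or below zero.
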(event `self.ReceiveBeginPlay`
  (`KismetSystemLibrary.K2_SetTimer` null "UpdateTime" 1.0 true))

(fn `UpdateTime`
  (bind _stormtimeinsec (`self.StormTimeInSec`))
  (bind _calmtimeinsec (`self.CalmTimeInSec`))
  (switch `/Game/Data/E_PlayState` (`self.PlayState`)
    (:`NewEnumerator0`
      (if (> _calmtimeinsec 0)
        (`/Engine/EditorBlueprintResources/StandardMacros.DecrementInt` _calmtimeinsec)
        (else
          (set `self.PlayState` "NewEnumerator1")
          (bind _outactors (`GameplayStatics.GetAllActorsWithInterface` "/Game/Blueprints/Interfaces/BPI_PlayStateEvents.BPI_PlayStateEvents_C"))
          (for _array_element _outactors
            (message `/Game/Blueprints/Interfaces/BPI_PlayStateEvents.BeginStorm` _array_element)))))
    (:`NewEnumerator1`
      (if (> _stormtimeinsec 0)
        (`/Engine/EditorBlueprintResources/StandardMacros.DecrementInt` _stormtimeinsec)
        (else
          (set `self.PlayState` "NewEnumerator0")
          (bind _output_get (set `self.Difficulty` (+ (`self.Difficulty`) 0.1)))
          (set `self.CalmTimeInSec` (- (`self.CalmTimeInSec`) (* 10 _output_get)))
          (set `self.StormTimeInSec` (+ (`self.StormTimeInSec`) (* 5 _output_get)))
          (bind _outactors_2 (`GameplayStatics.GetAllActorsWithInterface` "/Game/Blueprints/Interfaces/BPI_PlayStateEvents.BPI_PlayStateEvents_C"))
          (for _array_element_2 _outactors_2
            (message `/Game/Blueprints/Interfaces/BPI_PlayStateEvents.BeginCalm` _array_element_2)))))))

(fn `UserConstructionScript`)
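; Player controller that creates the game HUD and keeps the player's Wood, Stone and Iron resource totals.
; On BeginPlay it creates a WBP_HUD widget, stores the reference and adds it to the viewport.
; AddResourceAmount switches on resource type to increase the matching total, but only Wood changes are pushed to the HUD; Stone and Iron update silently.
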(event `self.ReceiveBeginPlay`
  (bind _returnvalue (`|CreateWidget` "/Game/UI/Widgets/WBP_HUD.WBP_HUD_C"))
  (bind _output_get (set `self.HUDRef` _returnvalue))
  (`UserWidget.AddToViewport` _output_get 0))

(fn `AddResourceAmount`
  (params (ResourceType :type "/Game/Data/E_Resources Enum" :default "NewEnumerator0") (ResourceAmount :type Integer))
  (locals (Amount :type Integer))
  (set `local.Amount` ResourceAmount)
  (switch `/Game/Data/E_Resources` ResourceType
    (:`NewEnumerator0`
      (bind _output_get (set `self.Wood` (+ (`self.Wood`) (`local.Amount`))))
      (`/Game/UI/Widgets/WBP_HUD.UpdateWoodCount` (`self.HUDRef`) _output_get))
    (:`NewEnumerator1`
      (set `self.Stone` (+ (`self.Stone`) (`local.Amount`))))
    (:`NewEnumerator2`
      (set `self.Iron` (+ (`self.Iron`) (`local.Amount`))))))

(fn `UserConstructionScript`)
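; Interactable campfire that is built with stone, lit and refueled with wood from the player's resources, and warms nearby pawns.
; Interacting spends one resource per step and raises WoodAmount, while a looping timer started on lighting burns it down.
; Wood thresholds select fire levels that scale the smoke effect and TemperatureArea radius, whose overlaps toggle the warm state on the player controller.
; Tick prints the wood amount for debugging.
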(event `self.ReceiveTick`
  (params (DeltaSeconds :type "Float (single-precision)"))
  (`KismetSystemLibrary.PrintString` (`KismetStringLibrary.Conv_DoubleToString` (`self.WoodAmount`)) true true (struct :`R` 1.0 :`G` 0.381344 :`A` 1.0) 0.0))

(event `self.ReceiveBeginPlay`
  (`parent.ReceiveBeginPlay`))

(event `/Game/Blueprints/Interfaces/BPI_Interaction.Interact`
  (bind _playercontrollerref (`self.PlayerControllerRef`))
  ;[0.1085 0.3525 1] Interact
  (if (`self.bIsFireOn`)
    (if (`/Game/Blueprints/Core/BP_ICBW_PlayerController.HasResource` (`self.PlayerControllerRef`) "NewEnumerator0")
      (`self.FuelFire`))
    (elif (and (`/Game/Blueprints/Core/BP_ICBW_PlayerController.HasResource` _playercontrollerref "NewEnumerator0") (`/Game/Blueprints/Core/BP_ICBW_PlayerController.HasResource` _playercontrollerref "NewEnumerator1"))
      (`self.LightFire`))))

(event `self.TemperatureArea.OnComponentBeginOverlap`
  (params (OverlappedComponent :type "PrimitiveComponent Object Reference") (OtherActor :type "Actor Object Reference") (OtherComp :type "PrimitiveComponent Object Reference") (OtherBodyIndex :type Integer) (bFromSweep :type Boolean) (SweepResult :type "HitResult Structure (by ref)"))
  ;[0.1479 1 0.1009] Temperature Area
  (cast `/Game/Blueprints/Pawns/BP_BasePawn` OtherActor)
  (`/Game/Blueprints/Core/BP_ICBW_PlayerController.SetIsPawnWarm` (`self.PlayerControllerRef`) true))

(event `self.TemperatureArea.OnComponentEndOverlap`
  (params (OverlappedComponent :type "PrimitiveComponent Object Reference") (OtherActor :type "Actor Object Reference") (OtherComp :type "PrimitiveComponent Object Reference") (OtherBodyIndex :type Integer))
  ;[0.1479 1 0.1009] Temperature Area
  (cast `/Game/Blueprints/Pawns/BP_BasePawn` OtherActor)
  (`/Game/Blueprints/Core/BP_ICBW_PlayerController.SetIsPawnWarm` (`self.PlayerControllerRef`) false))

(fn `CheckWoodAmount`
  (switch `int` (`self.FireLevel`)
    (:`1`
      (if (<= (`self.WoodAmount`) 0.0)
        (`self.PutOutFire`)))
    (:`2`
      (if (< (`self.WoodAmount`) 2.5)
        (`self.SetFireLevel` 1)))
    (:`3`
      (if (< (`self.WoodAmount`) 4.5)
        (`self.SetFireLevel` 2)))))

(fn `ConsumeWood`
  (set `self.WoodAmount` (- (`self.WoodAmount`) (`self.ConsumedWoodPerSec`)))
  (`self.CheckWoodAmount`))

(fn `FuelFire`
  (`/Game/Blueprints/Core/BP_ICBW_PlayerController.UpdateResourceAmount` (`self.PlayerControllerRef`) "NewEnumerator0" -1)
  (bind _result (`/Engine/EditorBlueprintResources/StandardMacros.IncrementFloat` (`self.WoodAmount`))
    (:`  `
      (if (> _result 4.0)
        (`self.SetFireLevel` 3)
        (elif (> (`self.WoodAmount`) 2.0)
          (`self.SetFireLevel` 2))))))

(fn `LightFire`
  (bind _playercontrollerref (`self.PlayerControllerRef`))
  (if (`self.bHasStone`)
    (`/Game/Blueprints/Core/BP_ICBW_PlayerController.UpdateResourceAmount` _playercontrollerref "NewEnumerator0" -1)
    (`/Engine/EditorBlueprintResources/StandardMacros.IncrementFloat` (`self.WoodAmount`)
      (:`  `
        (`self.SetFireLevel` 1)))
    (else
      (`/Game/Blueprints/Core/BP_ICBW_PlayerController.UpdateResourceAmount` _playercontrollerref "NewEnumerator1" -1)
      (set `self.bHasStone` true)
      (`BillboardComponent.SetSprite` (`self.Billboard`) "/Game/UI/Icons/I_Wood.I_Wood"))))

(fn `PutOutFire`
  (`self.SetFireLevel` 0)
  (`KismetSystemLibrary.K2_ClearAndInvalidateTimerHandle` (`self.BurningTimer`)))

(fn `SetFireLevel`
  (params (Level :type Integer))
  (bind _output_get (set `self.FireLevel` Level))
  (switch `int` _output_get
    (:`0`
      (`ActorComponent.Deactivate` (`self.Fire`))
      (`SceneComponent.SetVisibility` (`self.PointLight`) false false)
      (set `self.WoodAmount` 0.0)
      (set `self.bIsFireOn` false)
      (`SphereComponent.SetSphereRadius` (`self.TemperatureArea`) 0.0 true))
    (:`1`
      (`ActorComponent.Activate` (`self.Fire`) false)
      (`SceneComponent.SetVisibility` (`self.PointLight`) false false)
      (set `self.bHasStone` false)
      (set `self.bIsFireOn` true)
      (`NiagaraComponent.SetVariableFloat` (`self.Fire`) "SmokeMeshScale" 1.0)
      (`SphereComponent.SetSphereRadius` (`self.TemperatureArea`) 200.0 true)
      (bind _returnvalue (`KismetSystemLibrary.K2_SetTimerDelegate` (`|CreateDelegate` :!event `ConsumeWood`) 1.0 true))
      (set `self.BurningTimer` _returnvalue))
    (:`2`
      (`NiagaraComponent.SetVariableFloat` (`self.Fire`) "SmokeMeshScale" 2.0)
      (`SphereComponent.SetSphereRadius` (`self.TemperatureArea`) 400.0 true))
    (:`3`
      (`NiagaraComponent.SetVariableFloat` (`self.Fire`) "SmokeMeshScale" 3.0)
      (`SphereComponent.SetSphereRadius` (`self.TemperatureArea`) 800.0 true))))

(fn `UserConstructionScript`)
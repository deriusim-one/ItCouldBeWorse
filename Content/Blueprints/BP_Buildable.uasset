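; BP_Buildable is an interactable build site that consumes an ordered list of resources and replaces itself with the finished actor.
; Each interaction spends one unit of the current wood, stone or iron requirement and advances the index, destroying itself and spawning ActorToSpawnClass when the list completes.
; It sets a resource or failure sound around the parent Interact call.
; A billboard, revealed on pawn overlap, shows the needed resource, in black-and-white when the player lacks it.
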(event `/Game/Blueprints/Interfaces/BPI_Interaction.Interact`
  (bind _resourcesindex (`self.ResourcesIndex`))
  (if (`/Game/Blueprints/Core/BP_ICBW_PlayerController.HasResource` (`self.PlayerControllerRef`) (`self.GetCurrentResourceNeeded`))
    (`self.SetSoundBasedOnCurrentResource`)
    (`parent.Interact`)
    (`/Game/Blueprints/Core/BP_ICBW_PlayerController.UpdateResourceAmount` (`self.PlayerControllerRef`) (`self.GetCurrentResourceNeeded`) -1)
    (`/Engine/EditorBlueprintResources/StandardMacros.IncrementInt` _resourcesindex
      (:`  `
        (if (== _resourcesindex (`KismetArrayLibrary.Array_Length` (`.ResourcesNeeded_4_678A93364BBBD6504E5ED38C695DDA03` (break `/Game/Data/F_Buildings` (`|GetArrayItem` (`self.BuildingLevel`) (`self.BuildingLevelIndex`))))))
          (`self.K2_DestroyActor`)
          (`|SpawnActorFromClass` (`self.ActorToSpawnClass`) (`self.GetTransform`) "Undefined" "MultiplyWithRoot" null null)
          (else
            (`self.SetBillboardBasedOnCurrentResource`)))))
    (else
      (set `self.Sound` "/Engine/EditorSounds/Notifications/CompileFailed_Cue.CompileFailed_Cue")
      (`parent.Interact`))))

(event `self.InteractionSphere.OnComponentBeginOverlap`
  (params (OverlappedComponent :type "PrimitiveComponent Object Reference") (OtherActor :type "Actor Object Reference") (OtherComp :type "PrimitiveComponent Object Reference") (OtherBodyIndex :type Integer) (bFromSweep :type Boolean) (SweepResult :type "HitResult Structure (by ref)"))
  (cast `/Game/Blueprints/Pawns/BP_BasePawn` OtherActor)
  (`self.SetBillboardBasedOnCurrentResource`)
  (`SceneComponent.SetVisibility` (`self.Billboard`) true false))

(fn `GetCurrentResourceNeeded`
  (returns (ResourceType :type "/Game/Data/E_Resources Enum"))
  (return (`|GetArrayItem` (`.ResourcesNeeded_4_678A93364BBBD6504E5ED38C695DDA03` (break `/Game/Data/F_Buildings` (`|GetArrayItem` (`self.BuildingLevel`) (`self.BuildingLevelIndex`)))) (`self.ResourcesIndex`))))

(fn `SetBillboardBasedOnCurrentResource`
  (bind _resourcetype (`self.GetCurrentResourceNeeded`))
  (bind _hasresource (`/Game/Blueprints/Core/BP_ICBW_PlayerController.HasResource` (`self.PlayerControllerRef`) _resourcetype))
  (`BillboardComponent.SetSprite` (`self.Billboard`) (select `/Game/Data/E_Resources` _resourcetype :`NewEnumerator0` (select `bool` _hasresource :`false` "/Game/UI/Icons/I_Wood_BW.I_Wood_BW" :`true` "/Game/UI/Icons/I_Wood.I_Wood" :!type "Texture2D Object Reference") :`NewEnumerator1` (select `bool` _hasresource :`false` "/Game/UI/Icons/I_Stone_BW.I_Stone_BW" :`true` "/Game/UI/Icons/I_Stone.I_Stone" :!type "Texture2D Object Reference") :`NewEnumerator2` (select `bool` _hasresource :`false` "/Game/UI/Icons/I_Iron_BW.I_Iron_BW" :`true` "/Game/UI/Icons/I_Iron.I_Iron" :!type "Texture2D Object Reference"))))

(fn `SetSoundBasedOnCurrentResource`
  (set `self.Sound` (select `/Game/Data/E_Resources` (`self.GetCurrentResourceNeeded`) :`NewEnumerator0` "/Game/Sounds/SFX_Wood_Cue.SFX_Wood_Cue" :`NewEnumerator1` "/Game/Sounds/SFX_Stone_Cue.SFX_Stone_Cue" :`NewEnumerator2` "/Game/Sounds/SFX_Iron_Cue.SFX_Iron_Cue" :!type "SoundCue Object Reference")))

(fn `UserConstructionScript`
  (`parent.UserConstructionScript`)
  (`self.SetBillboardBasedOnCurrentResource`))
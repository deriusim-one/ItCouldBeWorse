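; BP_Resource is a Wood or Stone resource pickup actor that disappears when a pawn touches it.
; The construction script picks the static mesh from ResourceType and Units, with three plank tiers for wood and two tiers for stone.
; Overlap of the collision sphere with a BP_BasePawn prints a debug string and destroys the actor.
; It does not credit the resource to the player, and a player controller cast sits unconnected.
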(event `self.SphereCollision.OnComponentBeginOverlap`
  (params (OverlappedComponent :type "PrimitiveComponent Object Reference") (OtherActor :type "Actor Object Reference") (OtherComp :type "PrimitiveComponent Object Reference") (OtherBodyIndex :type Integer) (bFromSweep :type Boolean) (SweepResult :type "HitResult Structure (by ref)"))
  (cast `/Game/Blueprints/Pawns/BP_BasePawn` OtherActor)
  (`KismetSystemLibrary.PrintString` "Hello")
  ;[1 1 1] Comment
  (`self.K2_DestroyActor`))

(fn `UserConstructionScript`
  (bind _staticmesh (`self.StaticMesh`))
  (bind _staticmesh_2 (`self.StaticMesh`))
  (switch `/Game/Data/E_Resources` (`self.ResourceType`)
    (:`NewEnumerator0`
      (if (< (`self.Units`) 2)
        (`StaticMeshComponent.SetStaticMesh` _staticmesh_2 "/Game/Meshes/SM_Resource_Planks_A.SM_Resource_Planks_A")
        (elif (< (`self.Units`) 4)
          (`StaticMeshComponent.SetStaticMesh` _staticmesh_2 "/Game/Meshes/SM_Resource_Planks_B.SM_Resource_Planks_B")
          (else
            (`StaticMeshComponent.SetStaticMesh` _staticmesh_2 "/Game/Meshes/SM_Resource_Planks_C.SM_Resource_Planks_C")))))
    (:`NewEnumerator1`
      (if (< (`self.Units`) 2)
        (`StaticMeshComponent.SetStaticMesh` _staticmesh "/Game/Meshes/SM_Resource_Stone_A.SM_Resource_Stone_A")
        (else
          (`StaticMeshComponent.SetStaticMesh` _staticmesh "/Game/Meshes/SM_Resource_Stone_B.SM_Resource_Stone_B"))))))
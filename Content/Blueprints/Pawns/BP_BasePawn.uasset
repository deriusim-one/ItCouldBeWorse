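; Base player pawn that provides top-down movement and interaction through Enhanced Input.
; BeginPlay caches the BP_ICBW_PlayerController and adds the IMC_TopDown_Motion mapping context to it.
; IA_Move drives movement input along right and forward vectors derived from control rotation.
; IA_Interact sends InteractMessage to the first overlapping actor only, if it implements BPI_Interaction.
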(event `self.ReceiveBeginPlay`
  (bind _asbp_icbw_player_controller (cast `/Game/Blueprints/Core/BP_ICBW_PlayerController` (`GameplayStatics.GetPlayerController` 0)))
  (bind _output_get (set `self.PlayerControllerRef` _asbp_icbw_player_controller))
  (`EnhancedInputSubsystemInterface.AddMappingContext` (pcsubsystem `EnhancedInputLocalPlayerSubsystem` _output_get) "/Game/Input/IMC_TopDown_Motion.IMC_TopDown_Motion" 0 (struct)))

(event `EnhancedInput|/Game/Input/Action/IA_Move`
  (params (ActionValue :type "Vector2D Structure") (ElapsedSeconds :type "Float (double-precision)") (TriggeredSeconds :type "Float (double-precision)") (InputAction :type "InputAction Object Reference" :default "/Game/Input/Action/IA_Move.IA_Move"))
  (bind (_returnvalue_roll _returnvalue_pitch _returnvalue_yaw) (`KismetMathLibrary.BreakRotator` (`self.GetControlRotation`)))
  (bind (_returnvalue_roll_2 _returnvalue_pitch_2 _returnvalue_yaw_2) (`KismetMathLibrary.BreakRotator` (`self.GetControlRotation`)))
  ;[0.02843 0.2159 0.8469] Movement
  (:`Triggered`
    (`self.AddMovementInput` (`KismetMathLibrary.GetRightVector` (`KismetMathLibrary.MakeRotator` _returnvalue_roll_2 0.0 _returnvalue_yaw_2)) ActionValue_X)
    (`self.AddMovementInput` (`KismetMathLibrary.GetForwardVector` (`KismetMathLibrary.MakeRotator` 0.0 0.0 _returnvalue_yaw)) ActionValue_Y)))

(event `EnhancedInput|/Game/Input/Action/IA_Interact`
  (params (ActionValue :type Boolean) (ElapsedSeconds :type "Float (double-precision)") (TriggeredSeconds :type "Float (double-precision)") (InputAction :type "InputAction Object Reference" :default "/Game/Input/Action/IA_Interact.IA_Interact"))
  (bind _output (`|GetArrayItem` (`self.GetOverlappingActors` null)))
  (:`Triggered`
    (if (`KismetSystemLibrary.DoesImplementInterface` _output "/Game/Blueprints/Interfaces/BPI_Interaction.BPI_Interaction_C")
      (message `/Game/Blueprints/Interfaces/BPI_Interaction.Interact` _output))))

(fn `UserConstructionScript`)